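; BP_RoomGenerator builds modular rooms in the construction script from the RoomsInfo array, unless Lock freezes the instance.
; Initialization clears floor, wall and ceiling instanced meshes, then places each room by its origin, the first at zero.
; Rooms get tiled floors, stacked mirrored walls, and a tiled box or single scaled curved ceiling on one shared component.
; RemoveChunks deletes walls within a sphere but is never called here; PipeSpawning is empty.
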(fn `CeilingCreation`
  (params (`Room Origin` :type "Vector Structure") (`Floor Y` :type Integer) (`Floor X` :type Integer) (`Wall Height` :type Integer) (`Ceiling Shape` :type "/Game/PCFTest/Data/CeilingShapes Enum" :default "NewEnumerator0"))
  (bind _returnvalue (`KismetMathLibrary.Conv_IntToDouble` `Floor Y`))
  (bind _ceiling (`self.Ceiling`))
  (switch `/Game/PCFTest/Data/CeilingShapes` `Ceiling Shape`
    (:`NewEnumerator0`
      ;[1 1 1] Box Ceiling
      (`StaticMeshComponent.SetStaticMesh` (`self.Ceiling`) (`self.BoxCeilingMesh`))
      (for _index (range `Floor Y`)
        (for _index_2 (range `Floor X`)
          (`InstancedStaticMeshComponent.AddInstance` (`self.Ceiling`) (`KismetMathLibrary.MakeTransform` (+ `Room Origin` (`KismetMathLibrary.MakeVector` (* _index_2 100.0) (* _index 100.0) (* `Wall Height` 100.0))))))))
    (:`NewEnumerator1`
      ;[1 1 1] Curved Ceiling
      (`StaticMeshComponent.SetStaticMesh` _ceiling (`self.CurvedCeilingMesh`))
      (`InstancedStaticMeshComponent.AddInstance` _ceiling (`KismetMathLibrary.MakeTransform` (+ `Room Origin` (`KismetMathLibrary.MakeVector` 0.0 0.0 (* `Wall Height` 100.0))) (struct) (`KismetMathLibrary.MakeVector` (`KismetMathLibrary.Conv_IntToDouble` `Floor X`) _returnvalue (/ _returnvalue 2.0)))))))

(fn `CreateRoom`
  (params (`Room Origin` :type "Vector Structure") (`Floor X` :type Integer) (`Floor Y` :type Integer) (`Wall Height` :type Integer) (`Ceiling Shape` :type "/Game/PCFTest/Data/CeilingShapes Enum" :default "NewEnumerator0"))
  (`|ExecutionSequence`
    (:`then_0`
      (`self.FloorCreation` `Floor X` `Floor Y` `Room Origin`))
    (:`then_1`
      (`self.WallCreation` `Room Origin` `Wall Height` `Floor X` `Floor Y`))
    (:`then_2`
      ;[1 1 1] Ceiling
      (`self.CeilingCreation` `Room Origin` `Floor Y` `Floor X` `Wall Height` `Ceiling Shape`))))

(fn `FloorCreation`
  (params (`Floor X` :type Integer) (`Floor Y` :type Integer) (`Room Origin` :type "Vector Structure"))
  (for _index (range `Floor Y`)
    (for _index_2 (range `Floor X`)
      (`InstancedStaticMeshComponent.AddInstance` (`self.Floors`) (`KismetMathLibrary.MakeTransform` (+ `Room Origin` (`KismetMathLibrary.MakeVector` (* _index_2 100.0) (* _index 100.0))))))))

(fn `Initialization`
  (bind _returnvalue (`KismetArrayLibrary.Array_Length` (`self.RoomsInfo`)))
  (bind (_floorx _floory _wallheight _ceilingtype) (break `/Game/PCFTest/Data/RoomInfo` (`|GetArrayItem` (`self.RoomsInfo`))))
  ;[1 1 1] Clears all the previous instances
  (`InstancedStaticMeshComponent.ClearInstances` (`self.Floors`))
  (`InstancedStaticMeshComponent.ClearInstances` (`self.Walls`))
  (`InstancedStaticMeshComponent.ClearInstances` (`self.Ceiling`))
  (`|ExecutionSequence`
    (:`then_0`
      (set `self.Offset` 0))
    (:`then_1`
      ;[1 1 1] First Room
      (`self.CreateRoom` (0.0 0.0 0.0) _floorx _floory _wallheight _ceilingtype))
    (:`then_2`
      (if (> _returnvalue 1)
        (for _index (range 1 _returnvalue)
          (bind (_floorx_2 _floory_2 _wallheight_2 _ceilingtype_2 _origin) (break `/Game/PCFTest/Data/RoomInfo` (`|GetArrayItem` (`self.RoomsInfo`) _index)))
          ;[1 1 1] Calc Origin based on Previous room
          (`self.CreateRoom` _origin _floorx_2 _floory_2 _wallheight_2 _ceilingtype_2))))))

(fn `PipeSpawning`)

(fn `RemoveChunks`
  (params (Center :type "Vector Structure") (Extent :type "Vector Structure") (Radius :type "Float (double-precision)"))
  (bind _walls (`self.Walls`))
  (for _array_element (`InstancedStaticMeshComponent.GetInstancesOverlappingSphere` _walls Center Radius true) :!label _label
    (bind _returnvalue (`InstancedStaticMeshComponent.RemoveInstance` _walls _array_element))
    (if _returnvalue
      (goto _label)))
  (return))

(fn `UserConstructionScript`
  ;[1 0 0.1187] If you like what you see, lock me on the instance!
  (if (not (`self.Lock`))
    ;[1 1 1] Meat & Potatoes
    (`self.Initialization`)))

(fn `WallCreation`
  (params (`Room Origin` :type "Vector Structure") (`Wall Height` :type Integer) (`Floor X` :type Integer) (`Floor Y` :type Integer))
  ;[1 1 1] Wall height
  (for _index (range `Wall Height`)
    ;[1 1 1] Both X Walls 0 and 1
    (for _index_2 (range 2)
      ;[1 1 1] X
      (for _index_3 (range `Floor X`)
        (bind _returnvalue (not (`KismetMathLibrary.Conv_IntToBool` _index_2)))
        (bind _returnvalue_2 (`KismetMathLibrary.MakeVector` (* _index_3 (`self.UnitLength`)) (`KismetMathLibrary.SelectFloat` 0.0 (* `Floor Y` (`self.UnitLength`)) _returnvalue)))
        (bind _returnvalue_3 (* _index (`self.UnitLength`)))
        (`InstancedStaticMeshComponent.AddInstance` (`self.Walls`) (`KismetMathLibrary.MakeTransform` (+ `Room Origin` (`KismetMathLibrary.MakeVector` (.x (`KismetMathLibrary.SelectVector` _returnvalue_2 (- _returnvalue_2 (`KismetMathLibrary.MakeVector` (* (`self.UnitLength`) -1.0))) _returnvalue)) (.y (`KismetMathLibrary.SelectVector` _returnvalue_2 (- _returnvalue_2 (`KismetMathLibrary.MakeVector` (* (`self.UnitLength`) -1.0))) _returnvalue)) _returnvalue_3)) (`KismetMathLibrary.SelectRotator` (struct) (struct :`Yaw` 180.0) _returnvalue))))
      ;[1 1 1] Y
      (for _index_4 (range `Floor Y`)
        (bind _returnvalue_4 (not (`KismetMathLibrary.Conv_IntToBool` _index_2)))
        (bind _returnvalue_5 (`KismetMathLibrary.MakeVector` (`KismetMathLibrary.SelectFloat` 0.0 (* `Floor X` (`self.UnitLength`)) _returnvalue_4) (* _index_4 (`self.UnitLength`))))
        (`InstancedStaticMeshComponent.AddInstance` (`self.Walls`) (`KismetMathLibrary.MakeTransform` (+ `Room Origin` (`KismetMathLibrary.MakeVector` (.x (`KismetMathLibrary.SelectVector` (- _returnvalue_5 (`KismetMathLibrary.MakeVector` 0.0 (* (`self.UnitLength`) -1.0))) _returnvalue_5 _returnvalue_4)) (.y (`KismetMathLibrary.SelectVector` (- _returnvalue_5 (`KismetMathLibrary.MakeVector` 0.0 (* (`self.UnitLength`) -1.0))) _returnvalue_5 _returnvalue_4)) _returnvalue_3)) (`KismetMathLibrary.SelectRotator` (struct :`Yaw` 270.0) (struct :`Yaw` 90.0) _returnvalue_4)))))))