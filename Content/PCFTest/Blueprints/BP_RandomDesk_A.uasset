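; Desk prop Blueprint that randomizes its look in the Construction Script, with no active runtime logic.
; Each of four drawers gets a random Y slide, with nested coin flips leaving most closed.
; One of two chairs is shown.
; Desk props are hidden, then one of two monitor-based layouts with random picks is revealed, plus either a phone or a file.
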(fn `RandomChair`
  (bind _array (`|MakeArray` (`self.OS_ChairWhite_StaticMeshComponent0`) (`self.OS_ChairBlack_StaticMeshComponent0`)))
  (`SceneComponent.SetVisibility` _array false false)
  (`SceneComponent.SetVisibility` (`KismetArrayLibrary.Array_Random` _array) true false))

(fn `RandomDeskProps`
  (locals (finalArray :type "Array of StaticMeshComponent Object Reference"))
  (bind _os_monitor_c_staticmeshcomponent0 (`self.OS_Monitor_C_StaticMeshComponent0`))
  (bind _os_monitor_a_staticmeshcomponent0 (`self.OS_Monitor_A_StaticMeshComponent0`))
  (bind _os_phone_staticmeshcomponent0 (`self.OS_Phone_StaticMeshComponent0`))
  (bind _os_file_b_staticmeshcomponent0 (`self.OS_File_B_StaticMeshComponent0`))
  (bind _os_radio_b_staticmeshcomponent0 (`self.OS_Radio_B_StaticMeshComponent0`))
  (bind _os_desklamp_staticmeshcomponent0 (`self.OS_DeskLamp_StaticMeshComponent0`))
  (bind _os_radio_c_staticmeshcomponent0 (`self.OS_Radio_C_StaticMeshComponent0`))
  (bind _os_monitor_d_staticmeshcomponent0 (`self.OS_Monitor_D_StaticMeshComponent0`))
  (bind _os_keyboard_staticmeshcomponent0 (`self.OS_Keyboard_StaticMeshComponent0`))
  (bind _os_monitor_f_staticmeshcomponent0 (`self.OS_monitor_F_StaticMeshComponent0`))
  (bind _os_monitor_e_staticmeshcomponent0 (`self.OS_Monitor_E_StaticMeshComponent0`))
  (`SceneComponent.SetVisibility` (`|MakeArray` _os_monitor_a_staticmeshcomponent0 _os_monitor_c_staticmeshcomponent0 _os_keyboard_staticmeshcomponent0 _os_radio_b_staticmeshcomponent0 _os_desklamp_staticmeshcomponent0 _os_radio_c_staticmeshcomponent0 _os_monitor_d_staticmeshcomponent0 _os_monitor_f_staticmeshcomponent0 _os_monitor_e_staticmeshcomponent0 _os_phone_staticmeshcomponent0 _os_file_b_staticmeshcomponent0) false false)
  (bind _output_get (set `local.finalArray` (select `int` (`KismetMathLibrary.RandomIntegerInRange` 0 1) :`0` (`|MakeArray` (`KismetArrayLibrary.Array_Random` (`|MakeArray` _os_monitor_a_staticmeshcomponent0 _os_monitor_c_staticmeshcomponent0)) _os_keyboard_staticmeshcomponent0) :`1` (`|MakeArray` (`KismetArrayLibrary.Array_Random` (`|MakeArray` _os_radio_b_staticmeshcomponent0 _os_desklamp_staticmeshcomponent0 _os_radio_c_staticmeshcomponent0 _os_monitor_d_staticmeshcomponent0)) _os_monitor_f_staticmeshcomponent0 _os_monitor_e_staticmeshcomponent0))))
  (`KismetArrayLibrary.Array_Append` _output_get (`|MakeArray` (`KismetArrayLibrary.Array_Random` (`|MakeArray` _os_phone_staticmeshcomponent0 _os_file_b_staticmeshcomponent0))))
  (`SceneComponent.SetVisibility` _output_get true false))

(fn `RandomDrawerPositions`
  (bind _returnvalue (`KismetMathLibrary.RandomBool`))
  (for _array_element (`|MakeArray` (`self.OS_Desk_Drawer_A_StaticMeshComponent0`) (`self.OS_Desk_Drawer_B_StaticMeshComponent0`) (`self.OS_Desk_Drawer_C_StaticMeshComponent0`) (`self.OS_Desk_Drawer_D_StaticMeshComponent0`))
    (`SceneComponent.K2_SetRelativeLocation` _array_element (`KismetMathLibrary.MakeVector` 0.0 (`KismetMathLibrary.SelectFloat` (`KismetMathLibrary.SelectFloat` (`KismetMathLibrary.RandomFloatInRange` 0.0 15.0) 0.0 _returnvalue) 0.0 _returnvalue)) false false)))

(fn `UserConstructionScript`
  (`self.RandomDrawerPositions`)
  (`self.RandomChair`)
  (`self.RandomDeskProps`))