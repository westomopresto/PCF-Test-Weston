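; BP_WallCutter is a placeable box that cuts openings in the instanced walls built by BP_RoomGenerator.
; All work runs in the Construction Script; the first cutter returned by GetAllActorsOfClass re-initializes every room generator, so only one instance triggers that reset.
; Each cutter then box-overlaps WorldDynamic instanced mesh components tagged "wall" and passes its box transform and extent to the owning generator's RemoveChunks.
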(fn `UserConstructionScript`
  (`|ExecutionSequence`
    (:`then_0`
      (bind _outactors (`GameplayStatics.GetAllActorsOfClass` "BP_WallCutter_C"))
      (if (== (`|GetArrayItem` _outactors) self)
        (bind _outactors_2 (`GameplayStatics.GetAllActorsOfClass` "/Game/PCFTest/Blueprints/BP_RoomGenerator.BP_RoomGenerator_C"))
        (for _array_element _outactors_2
          (`/Game/PCFTest/Blueprints/BP_RoomGenerator.Initialization` _array_element))))
    (:`then_1`
      (bind _outcomponents (`KismetSystemLibrary.BoxOverlapComponents` (`self.K2_GetActorLocation`) (`BoxComponent.GetScaledBoxExtent` (`self.Box`)) (`|MakeArray` "ObjectTypeQuery2" :!type "EObjectTypeQuery Enum") "/Script/Engine.InstancedStaticMeshComponent"))
      (for _array_element_2 _outcomponents
        (bind _asbp_room_generator (cast `/Game/PCFTest/Blueprints/BP_RoomGenerator` (`ActorComponent.GetOwner` _array_element_2)))
        (if (`ActorComponent.ComponentHasTag` _array_element_2 "wall")
          (bind _asinstanced_static_mesh_component (cast `InstancedStaticMeshComponent` _array_element_2))
          (`/Game/PCFTest/Blueprints/BP_RoomGenerator.RemoveChunks` _asbp_room_generator _asinstanced_static_mesh_component (`SceneComponent.K2_GetComponentToWorld` (`self.Box`)) (`BoxComponent.GetScaledBoxExtent` (`self.Box`))))))))