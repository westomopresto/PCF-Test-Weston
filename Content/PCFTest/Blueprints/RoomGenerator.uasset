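; RoomGenerator is an editor-time generator that builds a rectangular grid of floor tile instances.
; The construction script clears the Floors instanced mesh component, then nested loops over FloorY and FloorX add unrotated, unit-scale instances at 100-unit spacing from the local origin.
; A Lock flag skips the rebuild, and the event graph has no active logic.
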(fn `UserConstructionScript`
  (if (not (`self.Lock`))
    (`InstancedStaticMeshComponent.ClearInstances` (`self.Floors`))
    (for _index (range (`self.FloorY`))
      (for _index_2 (range (`self.FloorX`))
        (`InstancedStaticMeshComponent.AddInstance` (`self.Floors`) (`KismetMathLibrary.MakeTransform` (`KismetMathLibrary.MakeVector` (* _index_2 100.0) (* _index 100.0))))))))